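; Shape_Cylinder_DM_BP is a destructible cylinder obstacle that breaks and damages a Car when the car enters its capsule.
; Each Car overlap applies radius damage with an impulse at the Destructible component's location.
; A DoOnce limits the Health deduction to the first hit, subtracting a fixed amount directly from the car.
; It then prints the car's status and quits the game if Health falls below zero.
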(event `self.Capsule.OnComponentBeginOverlap`
  (params (OverlappedComponent :type "PrimitiveComponent Object Reference") (OtherActor :type "Actor Object Reference") (OtherComp :type "PrimitiveComponent Object Reference") (OtherBodyIndex :type Integer) (bFromSweep :type Boolean) (SweepResult :type "HitResult Structure (by ref)"))
  (bind _destructible (`self.Destructible`))
  (bind _ascar (cast `/Game/BP/Car` OtherActor))
  (`|ExecutionSequence`
    (:`then_0`
      (`DestructibleComponent.ApplyRadiusDamage` _destructible 1.0 (`SceneComponent.K2_GetComponentLocation` _destructible) 10.0 100.0 true))
    (:`then_1`
      (`/Engine/EditorBlueprintResources/StandardMacros.DoOnce` false
        (:`Completed`
          (`KismetSystemLibrary.PrintString` "hit")
          (bind _output_get (set `/Game/BP/Car.Health` (- (`/Game/BP/Car.Health` _ascar) 0.25) _ascar))
          (`/Engine/EditorBlueprintResources/StandardMacros.CompareFloat` _output_get
            (:`>`
              (`KismetSystemLibrary.PrintString` "Im alive"))
            (:`<`
              (`KismetSystemLibrary.PrintString` "Game Over")
              (`KismetSystemLibrary.Delay` 0.0)
              (`KismetSystemLibrary.QuitGame` null "Quit"))))))))

(fn `UserConstructionScript`)