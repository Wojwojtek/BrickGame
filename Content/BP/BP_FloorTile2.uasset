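; Road tile for an endless car game that asks the BrickCars game mode to add another tile when the car overlaps EndTrigger, then destroys itself after a delay.
; GetAttachTransform exposes the AttachPoint transform.
; Helper functions gather spawn-point transforms into arrays and add child actors at random entries for blockers, obstacles, bins, batteries and props.
; The construction script is empty, and the event graph calls none of these helpers.
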(event `self.EndTrigger.OnComponentBeginOverlap`
  (params (OverlappedComponent :type "PrimitiveComponent Object Reference") (OtherActor :type "Actor Object Reference") (OtherComp :type "PrimitiveComponent Object Reference") (OtherBodyIndex :type Integer) (bFromSweep :type Boolean) (SweepResult :type "HitResult Structure (by ref)"))
  (cast `/Game/BP/Car` OtherActor)
  (bind _asbrick_cars (cast `/Game/BP/BrickCars` (`GameplayStatics.GetGameMode`)))
  (`/Game/BP/BrickCars.AddFloorTile` _asbrick_cars)
  (`KismetSystemLibrary.Delay` 2.0)
  (`self.K2_DestroyActor`))

(fn `ConstructionPropScript`
  (`self.SetSpawnProp`)
  (`self.SpawnMailBox`)
  (`self.SpawnLampPost`))

(fn `GetAttachTransform`
  (returns (AttachTransform :type "Transform Structure"))
  (return (`SceneComponent.K2_GetComponentToWorld` (`self.AttachPoint`))))

(fn `NewFunction_0`
  (params (self2 :type "SceneComponent Object Reference"))
  (returns (ReturnValue :type "Transform Structure"))
  (return (`SceneComponent.GetRelativeTransform` self2)))

(fn `NewFunction_1`
  (params (self2 :type "SceneComponent Object Reference"))
  (returns (ReturnValue :type "Transform Structure"))
  (return (`SceneComponent.GetRelativeTransform` self2)))

(fn `NewFunction_10`
  (params (self2 :type "SceneComponent Object Reference"))
  (returns (ReturnValue :type "Transform Structure"))
  (return (`SceneComponent.GetRelativeTransform` self2)))

(fn `NewFunction_11`)

(fn `NewFunction_12`
  (`self.SpawnLampPost`))

(fn `NewFunction_2`
  (params (self2 :type "SceneComponent Object Reference"))
  (returns (ReturnValue :type "Transform Structure"))
  (return (`SceneComponent.GetRelativeTransform` self2)))

(fn `NewFunction_3`
  (params (self2 :type "SceneComponent Object Reference")))

(fn `NewFunction_4`)

(fn `NewFunction_5`
  (params (self2 :type "SceneComponent Object Reference")))

(fn `NewFunction_6`
  (params (self2 :type "SceneComponent Object Reference"))
  (returns (ReturnValue :type "Transform Structure"))
  (return (`SceneComponent.GetRelativeTransform` self2)))

(fn `NewFunction_7`
  (params (self2 :type "SceneComponent Object Reference"))
  (returns (ReturnValue :type "Transform Structure"))
  (return (`SceneComponent.GetRelativeTransform` self2)))

(fn `NewFunction_8`
  (params (self2 :type "SceneComponent Object Reference"))
  (returns (ReturnValue :type "Transform Structure"))
  (return (`SceneComponent.GetRelativeTransform` self2)))

(fn `NewFunction_9`
  (params (self2 :type "SceneComponent Object Reference"))
  (returns (ReturnValue :type "Transform Structure"))
  (return (`SceneComponent.GetRelativeTransform` self2)))

(fn `SetSpawnObstacle`
  (bind _returnvalue (`self.NewFunction_6` (`self.SpawnPoint4`)))
  (bind _returnvalue_2 (`self.NewFunction_6` (`self.SpawnPoint5`)))
  (set `self.SpawnPoints` (`|MakeArray` _returnvalue _returnvalue_2)))

(fn `SetSpawnPoints`
  (bind _returnvalue (`self.NewFunction_0` (`self.SpawnPoint1`)))
  (bind _returnvalue_2 (`self.NewFunction_2` (`self.SpawnPoint5`)))
  (bind _returnvalue_3 (`self.NewFunction_2` (`self.SpawnPoint9`)))
  (set `self.SpawnPoints` (`|MakeArray` _returnvalue _returnvalue_2 _returnvalue_3)))

(fn `SetSpawnProp`
  (bind _returnvalue (`self.NewFunction_7` null))
  (bind _returnvalue_2 (`self.NewFunction_8` null))
  (bind _returnvalue_3 (`self.NewFunction_9` null))
  (bind _returnvalue_4 (`self.NewFunction_10` null))
  (set `self.SpawnProps` (`|MakeArray` _returnvalue _returnvalue_2 _returnvalue_3 _returnvalue_4)))

(fn `SpawnBatteryCollect`
  (bind _setspawnbattery (`self.SetSpawnBattery`))
  (`AddComponent|NODE_AddChildActorComponent-12` :`RelativeTransform` (`|GetArrayItem` _setspawnbattery (`KismetMathLibrary.RandomIntegerInRange` 0 (`KismetArrayLibrary.Array_LastIndex` _setspawnbattery)))))

(fn `SpawnBin`
  (bind _setspawnbin (`self.SetSpawnBin`))
  (`AddComponent|NODE_AddChildActorComponent-6` :`RelativeTransform` (`|GetArrayItem` _setspawnbin (`KismetMathLibrary.RandomIntegerInRange` 0 (`KismetArrayLibrary.Array_LastIndex` _setspawnbin)))))

(fn `SpawnBlocker1`
  (bind _spawnpoints (`self.SpawnPoints`))
  (`AddComponent|NODE_AddChildActorComponent-0` :`RelativeTransform` (`|GetArrayItem` _spawnpoints (`KismetMathLibrary.RandomIntegerInRange` 0 (`KismetArrayLibrary.Array_LastIndex` _spawnpoints)))))

(fn `SpawnLampPost`
  (bind _spawnprops (`self.SpawnProps`))
  (`AddComponent|NODE_AddChildActorComponent-10` :`RelativeTransform` (`|GetArrayItem` _spawnprops (`KismetMathLibrary.RandomIntegerInRange` 0 (`KismetArrayLibrary.Array_LastIndex` _spawnprops)))))

(fn `SpawnMailBox`
  (bind _spawnprops (`self.SpawnProps`))
  (`AddComponent|NODE_AddChildActorComponent-11` :`RelativeTransform` (`|GetArrayItem` _spawnprops (`KismetMathLibrary.RandomIntegerInRange` 0 (`KismetArrayLibrary.Array_LastIndex` _spawnprops)))))

(fn `SpawnObstacle`
  (bind _setspawnobstacle1 (`self.SetSpawnObstacle1`))
  (`AddComponent|NODE_AddChildActorComponent-3` :`RelativeTransform` (`|GetArrayItem` _setspawnobstacle1 (`KismetMathLibrary.RandomIntegerInRange` 0 (`KismetArrayLibrary.Array_LastIndex` _setspawnobstacle1)))))

(fn `SpawnObstacle2`
  (bind _spawnpoints (`self.SpawnPoints`))
  (`AddComponent|NODE_AddChildActorComponent-4` :`RelativeTransform` (`|GetArrayItem` _spawnpoints (`KismetMathLibrary.RandomIntegerInRange` 0 (`KismetArrayLibrary.Array_LastIndex` _spawnpoints)))))

(fn `SpawnObstacle3`
  (bind _spawnpoints (`self.SpawnPoints`))
  (`AddComponent|NODE_AddChildActorComponent-7` :`RelativeTransform` (`|GetArrayItem` _spawnpoints (`KismetMathLibrary.RandomIntegerInRange` 0 (`KismetArrayLibrary.Array_LastIndex` _spawnpoints)))))

(fn `SpawnObstacle4`
  (bind _spawnpoints (`self.SpawnPoints`))
  (`AddComponent|NODE_AddChildActorComponent-8` :`RelativeTransform` (`|GetArrayItem` _spawnpoints (`KismetMathLibrary.RandomIntegerInRange` 0 (`KismetArrayLibrary.Array_LastIndex` _spawnpoints)))))

(fn `SpawnPointBattery`
  (bind _returnvalue (`self.NewFunction_1` (`self.SpawnPoint7`)))
  (set `self.SetSpawnBattery` (`|MakeArray` _returnvalue)))

(fn `SpawnPointBin`
  (bind _returnvalue (`self.NewFunction_1` (`self.SpawnPoint2`)))
  (bind _returnvalue_2 (`self.NewFunction_0` (`self.SpawnPoint6`)))
  (bind _returnvalue_3 (`self.NewFunction_2` (`self.SpawnPoint10`)))
  (set `self.SetSpawnBin` (`|MakeArray` _returnvalue _returnvalue_2 _returnvalue_3)))

(fn `SpawnPointObstacle1`
  (bind _returnvalue (`self.NewFunction_2` (`self.SpawnPoint3`)))
  (bind _returnvalue_2 (`self.NewFunction_2` (`self.SpawnPoint4`)))
  (bind _returnvalue_3 (`self.NewFunction_2` (`self.SpawnPoint8`)))
  (set `self.SetSpawnObstacle1` (`|MakeArray` _returnvalue _returnvalue_3 _returnvalue_2)))

(fn `UserConstructionScript`)